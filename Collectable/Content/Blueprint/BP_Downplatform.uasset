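; Moving platform that travels toward a set end location while the first-person character is inside its trigger box, and returns when they leave.
; A timeline lerps the Start mesh from its BeginPlay position to EndLocation, with play rate derived from Duration and reversed on end overlap.
; The construction script applies the shared mesh, scale and rotation to Start and End, placing End at EndLocation to show the destination.
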(event `self.ReceiveBeginPlay`
  (set `self.start location` (`SceneComponent.RelativeLocation` (`self.start`))))

(event `self.Box.OnComponentBeginOverlap`
  (params (OverlappedComponent :type "PrimitiveComponent Object Reference") (OtherActor :type "Actor Object Reference") (OtherComp :type "PrimitiveComponent Object Reference") (OtherBodyIndex :type Integer) (bFromSweep :type Boolean) (SweepResult :type "HitResult Structure (by ref)"))
  (cast `/Game/FirstPerson/Blueprints/BP_FirstPersonCharacter` OtherActor)
  (`TimelineComponent.SetPlayRate` (`self.platformmoving`) (/ 1.0 (`self.duration`)))
  (bind (_direction _movetrack) (`Timeline|platformmoving` :!label _label)
    (:`Update`
      (`SceneComponent.K2_SetRelativeLocation` (`self.start`) (`KismetMathLibrary.VLerp` (`self.start location`) (`self.end location`) _movetrack) false false))))

(event `self.Box.OnComponentEndOverlap`
  (params (OverlappedComponent :type "PrimitiveComponent Object Reference") (OtherActor :type "Actor Object Reference") (OtherComp :type "PrimitiveComponent Object Reference") (OtherBodyIndex :type Integer))
  (cast `/Game/FirstPerson/Blueprints/BP_FirstPersonCharacter` OtherActor)
  (`TimelineComponent.SetPlayRate` (`self.platformmoving`) (/ 1.0 (`self.duration`)))
  (goto _label :!via `Reverse`))

(fn `UserConstructionScript`
  (bind _platformmesh (`self.Platformmesh`))
  (bind _end (`self.end`))
  (bind _start (`self.start`))
  (`StaticMeshComponent.SetStaticMesh` (`self.start`) _platformmesh)
  (`StaticMeshComponent.SetStaticMesh` _end _platformmesh)
  (`SceneComponent.SetRelativeScale3D` _start (`self.scale`))
  (`SceneComponent.SetRelativeScale3D` _end (`self.scale`))
  (`SceneComponent.K2_SetRelativeRotation` _start (`self.rotation`) false false)
  (`SceneComponent.K2_SetRelativeRotation` _end (`self.rotation`) false false)
  (`SceneComponent.K2_SetRelativeLocation` _end (`self.end location`) false false))