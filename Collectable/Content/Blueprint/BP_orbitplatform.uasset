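; BP_orbitplatform is an actor, apparently an orbiting platform, that travels along the spline of a BP_movingorbit actor.
; On BeginPlay it finds that actor by class and starts a timeline with play rate set to one over TimeToComplete.
; Each update maps the timeline track to distance along the spline, setting location in world space and rotation from the spline's local-space rotation.
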(event `self.ReceiveBeginPlay`
  (bind _returnvalue (`GameplayStatics.GetActorOfClass` "/Game/Blueprint/BP_movingorbit.BP_movingorbit_C"))
  (set `self.Spline Ref` _returnvalue)
  (`self.Move Object`))

(event `Move Object`
  (bind _spline (`/Game/Blueprint/BP_movingorbit.Spline` (`self.Spline Ref`)))
  (`TimelineComponent.SetPlayRate` (`self.Moveobject T`) (/ 1.0 (`self.Time to complete`)))
  (bind (_direction _flowtrack) (`Timeline|Moveobject T`)
    (:`Update`
      (bind _returnvalue (`KismetMathLibrary.Lerp` 0.0 (`SplineComponent.GetSplineLength` _spline) _flowtrack))
      (`self.K2_SetActorTransform` (`KismetMathLibrary.MakeTransform` (`SplineComponent.GetLocationAtDistanceAlongSpline` _spline _returnvalue "World") (`SplineComponent.GetRotationAtDistanceAlongSpline` _spline _returnvalue "Local"))))))

(fn `UserConstructionScript`)